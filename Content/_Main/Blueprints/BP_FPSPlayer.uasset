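; BP_FPSPlayer is the first-person player character, handling movement, mouse look, jumping and shooting through Enhanced Input.
; On BeginPlay it adds the input mapping context, casts the Weapon child actor to BP_BaseWeapon and links the two by reference.
; The weapon's gun mesh attaches to the FPS arms at a weapon-defined socket, and the weapon also supplies the Anim value.
; Shoot input forwards start and stop calls to the weapon.
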(event Input|EnhancedActionEvents|EnhancedInputActionIA_Move
  (params (ActionValue :type Vector%202D%20Structure) (ElapsedSeconds :type Float%20%28double-precision%29) (TriggeredSeconds :type Float%20%28double-precision%29) (InputAction :type Input%20Action%20Object%20Reference :default "/Game/_Main/Input/Actions/IA_Move.IA_Move"))
  ;[1 0 1] Controls player movement using WASD
  (Pawn|Input|AddMovementInput (Transformation|GetActorRightVector) (.x ActionValue) false)
  (Pawn|Input|AddMovementInput (Transformation|GetActorForwardVector) (.y ActionValue) false))

(event Input|EnhancedActionEvents|EnhancedInputActionIA_Look
  (params (ActionValue :type Vector%202D%20Structure) (ElapsedSeconds :type Float%20%28double-precision%29) (TriggeredSeconds :type Float%20%28double-precision%29) (InputAction :type Input%20Action%20Object%20Reference :default "/Game/_Main/Input/Actions/IA_Look.IA_Look"))
  ;[1 0 1] Control player look using Mouse
  (Pawn|Input|AddControllerYawInput (.x ActionValue))
  (Pawn|Input|AddControllerPitchInput (.y ActionValue)))

(event Input|EnhancedActionEvents|EnhancedInputActionIA_Jump
  (params (ActionValue :type Boolean) (ElapsedSeconds :type Float%20%28double-precision%29) (TriggeredSeconds :type Float%20%28double-precision%29) (InputAction :type Input%20Action%20Object%20Reference :default "/Game/_Main/Input/Actions/IA_Jump.IA_Jump"))
  ;[1 0 1] Controls player jumping using space bar
  (:Started
    (Character|Jump))
  (:Completed
    (Character|StopJumping)))

(event Input|EnhancedActionEvents|EnhancedInputActionIA_Shoot
  (params (ActionValue :type Boolean) (ElapsedSeconds :type Float%20%28double-precision%29) (TriggeredSeconds :type Float%20%28double-precision%29) (InputAction :type Input%20Action%20Object%20Reference :default "/Game/_Main/Input/Actions/IA_Shoot.IA_Shoot"))
  (bind _weapon_ref (Variables|Default|GetWeapon_REF))
  (:Started
    (Default|StartShooting _weapon_ref))
  (:Completed
    (Default|StopShooting _weapon_ref)))

(event EventBeginPlay
  (bind _returnvalue (Game|GetPlayerController 0))
  (bind _returnvalue_2 (PlayerController|LocalPlayerSubsystems|GetEnhancedInputLocalPlayerSubsystem _returnvalue))
  ;[0 0 1] BeginPlay
  (Utilities|IsValid _returnvalue_2
    (:Is%20Valid
      (Input|AddMappingContext _returnvalue_2 "/Game/_Main/Input/IMC_FPSGame.IMC_FPSGame" 0 "(bIgnoreAllPressedKeysUntilRelease=True,bForceImmediately=False,bNotifyUserSettings=False)")
      (bind _asbp_base_weapon (Utilities|Casting|CastToBP_BaseWeapon (Variables|/Script/Engine.ChildActorComponent|GetChildActor (Variables|Default|GetWeapon))))
      (bind _output_get (Variables|Default|SetWeapon_REF _asbp_base_weapon))
      (Variables|/Game/_Main/Blueprints/Weapons/BP_BaseWeapon.BP_BaseWeapon_C|SetPlayer_REF _output_get self)
      (Transformation|AttachComponentToComponent (Variables|/Game/_Main/Blueprints/Weapons/BP_BaseWeapon.BP_BaseWeapon_C|GetGunMesh (Variables|Default|GetWeapon_REF)) (Variables|Default|GetFPS_Arms) (Variables|/Game/_Main/Blueprints/Weapons/BP_BaseWeapon.BP_BaseWeapon_C|GetSocket (Variables|Default|GetWeapon_REF)) "SnapToTarget" "SnapToTarget" "SnapToTarget" true)
      (Variables|Default|SetAnim (Variables|/Game/_Main/Blueprints/Weapons/BP_BaseWeapon.BP_BaseWeapon_C|GetAnimation (Variables|Default|GetWeapon_REF))))))

(fn ConstructionScript)