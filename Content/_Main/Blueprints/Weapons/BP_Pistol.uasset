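; BP_Pistol is a pistol weapon Blueprint that extends a parent weapon class with its own firing behavior.
; When shooting starts, it plays a one-shot fire animation on the gun mesh and calls FireWeapon with its trace length and debug drawing off.
; It then plays a firing montage on the player's first-person arms, reusing a rifle montage.
; BeginPlay, overlap, Tick and construction only call the parent.
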(event EventBeginPlay
  (|CallParentFunction))

(event Collision|EventActorBeginOverlap
  (params (OtherActor :type Actor%20Object%20Reference))
  (|CallParentFunction OtherActor))

(event EventTick
  (params (DeltaSeconds :type Float%20%28single-precision%29))
  (|CallParentFunction DeltaSeconds))

(event EventStartShooting
  (Components|Animation|PlayAnimation (Variables|Default|GetGunMesh) "/Game/MilitaryWeapSilver/Weapons/Animations/Fire_Pistol_W.Fire_Pistol_W" false)
  (CallFunction|FireWeapon "None" (Variables|Default|GetTraceLength))
  (Animation|Montage|PlayMontage (Variables|/Game/_Main/Blueprints/BP_FPSPlayer.BP_FPSPlayer_C|GetFPS_Arms (Variables|Default|GetPlayer_REF)) "/Game/Man/Demo/Animations/FiringRifle_UE_Montage.FiringRifle_UE_Montage"))

(fn ConstructionScript
  (|CallParentFunction))