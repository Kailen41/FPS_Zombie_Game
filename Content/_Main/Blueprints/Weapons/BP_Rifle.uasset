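; Automatic rifle weapon Blueprint that fires repeatedly from the start of shooting until told to stop.
; StartShooting plays the gun's fire animation, calls FireWeapon with a trace length and plays the first-person arms montage.
; It then starts a looping timer at the fire rate, which repeats that sequence through FireRifle until StopShooting clears it.
; BeginPlay, overlap, Tick and construction only defer to the parent class.
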(event Custom|FireRifle
  (Components|Animation|PlayAnimation (Variables|Default|GetGunMesh) "/Game/MilitaryWeapSilver/Weapons/Animations/Fire_Rifle_W.Fire_Rifle_W" false)
  (CallFunction|FireWeapon "None" (Variables|Default|GetTraceLength))
  (Animation|Montage|PlayMontage (Variables|/Game/_Main/Blueprints/BP_FPSPlayer.BP_FPSPlayer_C|GetFPS_Arms (Variables|Default|GetPlayer_REF)) "/Game/Man/Demo/Animations/FiringRifle_UE_Montage.FiringRifle_UE_Montage"))

(event EventBeginPlay
  (|CallParentFunction))

(event Collision|EventActorBeginOverlap
  (params (OtherActor :type Actor%20Object%20Reference))
  (|CallParentFunction OtherActor))

(event EventTick
  (params (DeltaSeconds :type Float%20%28single-precision%29))
  (|CallParentFunction DeltaSeconds))

(event EventStartShooting
  (Components|Animation|PlayAnimation (Variables|Default|GetGunMesh) "/Game/MilitaryWeapSilver/Weapons/Animations/Fire_Rifle_W.Fire_Rifle_W" false)
  (CallFunction|FireWeapon "None" (Variables|Default|GetTraceLength))
  (Animation|Montage|PlayMontage (Variables|/Game/_Main/Blueprints/BP_FPSPlayer.BP_FPSPlayer_C|GetFPS_Arms (Variables|Default|GetPlayer_REF)) "/Game/Man/Demo/Animations/FiringRifle_UE_Montage.FiringRifle_UE_Montage"
    (:then
      (bind _returnvalue (Utilities|Time|SetTimerbyEvent (delegate Custom|FireRifle) (Variables|Default|GetFireRate) true))
      (Variables|Default|SetFireEvent _returnvalue))))

(event EventStopShooting
  (Utilities|Time|ClearandInvalidateTimerbyHandle (Variables|Default|GetFireEvent)))

(fn ConstructionScript
  (|CallParentFunction))