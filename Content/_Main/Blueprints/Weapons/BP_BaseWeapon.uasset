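; BP_BaseWeapon is a base weapon Blueprint with empty StartShooting and StopShooting events and a shared FireWeapon function.
; FireWeapon checks ammo, runs a Visibility line trace forward from the player's first-person camera over a given length, then decrements ammo.
; It sets a PlayAnimation flag according to whether ammo was available.
; The trace result is not used, so no damage or impact is applied here.
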(event Custom|StartShooting)

(event Custom|StopShooting)

(fn ConstructionScript)

(fn FireWeapon
  (params (TraceLength :type Float%20%28double-precision%29))
  (bind _player_ref (Variables|Default|GetPlayer_REF))
  (bind _fpscamera (Variables|/Game/_Main/Blueprints/BP_FPSPlayer.BP_FPSPlayer_C|GetFPSCamera _player_ref))
  (bind _returnvalue (Transformation|GetWorldLocation _fpscamera))
  (if (> (Variables|Default|GetCurrentAmmo) 0)
    (Variables|Default|SetPlayAnimation? true)
    (Collision|LineTraceByChannel _returnvalue (+ _returnvalue (* (Math|Vector|GetForwardVector _fpscamera) TraceLength)) "TraceTypeQuery1" false 0 "None")
    (Math|Integer|DecrementInt (Variables|Default|GetCurrentAmmo))
    (else
      (Variables|Default|SetPlayAnimation? false))))